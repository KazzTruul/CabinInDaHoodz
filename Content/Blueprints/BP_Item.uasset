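; BP_Item is a pickup item that adds itself to the player's inventory when interacted with.
; Its Interact event casts itself to BP_Interactable and calls Interact on it, then reaches the Inventory held by BP_GameMode.
; If ItemName is already there, it only prints a message; otherwise it adds the name and destroys the actor.
; Failed casts print debug strings.
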(event EventBeginPlay)

(event Collision|EventActorBeginOverlap
  (params (OtherActor :type Actor%20Object%20Reference)))

(event EventTick
  (params (DeltaSeconds :type Float%20%28single-precision%29)))

(event EventInteract
  (bind _asbp_interactable (Utilities|Casting|CastToBP_Interactable self)
    (:then
      (Default|Interact _asbp_interactable)
      (bind _asbp_game_mode (Utilities|Casting|CastToBP_GameMode (Game|GetGameMode))
        (:then
          (bind _contains (Default|CheckifContains (Variables|/Game/Blueprints/BP_GameMode.BP_GameMode_C|GetInventory _asbp_game_mode) (Variables|Default|GetItemName)))
          (if _contains
            (Development|PrintString "Item already in inventory")
            (else
              (bind _asbp_game_mode_2 (Utilities|Casting|CastToBP_GameMode (Game|GetGameMode))
                (:then
                  (Default|AddtoInventory (Variables|/Game/Blueprints/BP_GameMode.BP_GameMode_C|GetInventory _asbp_game_mode_2) (Variables|Default|GetItemName))
                  (Actor|DestroyActor))
                (:CastFailed
                  (Development|PrintString "Cast to BP_GameMode failed"))))))
        (:CastFailed
          (Development|PrintString "Cast to BP_GameMode failed"))))
    (:CastFailed
      (Development|PrintString "Cast to interactable failed"))))

(fn ConstructionScript)