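; BP_NonVRPlayer is the non-VR player pawn with look and move controls, taking over the first player controller's view on BeginPlay.
; Look axes add yaw and pitch input scaled by LookSpeed.
; Move axis events add input along yaw-only forward and right vectors from control rotation, scaled by MoveSpeed alone, without reading the axis value.
; SetLookSpeed and SetMoveSpeed expose both speeds for adjustment.
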(event EventBeginPlay
  (Game|Player|SetViewTargetwithBlend (Game|GetPlayerController 0) self 0.0 "VTBlend_Linear" 0.0 false))

(event Collision|EventActorBeginOverlap
  (params (OtherActor :type Actor%20Object%20Reference)))

(event EventTick
  (params (DeltaSeconds :type Float%20%28single-precision%29)))

(event Input|AxisEvents|InputAxisInputAxisUp
  (params (AxisValue :type Float%20%28single-precision%29))
  (Pawn|Input|AddControllerPitchInput (* AxisValue (Variables|Default|GetLookSpeed))))

(event Input|AxisEvents|InputAxisInputAxisRight
  (params (AxisValue :type Float%20%28single-precision%29))
  (Pawn|Input|AddControllerYawInput (* AxisValue (Variables|Default|GetLookSpeed))))

(event Input|AxisEvents|InputAxisInputMoveForward
  (params (AxisValue :type Float%20%28single-precision%29))
  (Pawn|Input|AddMovementInput (Math|Vector|GetForwardVector (Math|Rotator|MakeRotator 0.0 0.0 (.Yaw (Math|Rotator|BreakRotator (Pawn|GetControlRotation :!class /Script/Engine.Pawn))))) (Variables|Default|GetMoveSpeed) false))

(event Input|AxisEvents|InputAxisInputMoveRight
  (params (AxisValue :type Float%20%28single-precision%29))
  (Pawn|Input|AddMovementInput (Math|Vector|GetRightVector (Math|Rotator|MakeRotator 0.0 0.0 (.Yaw (Math|Rotator|BreakRotator (Pawn|GetControlRotation :!class /Script/Engine.Pawn))))) (Variables|Default|GetMoveSpeed) false))

(fn ConstructionScript)

(fn SetLookSpeed
  (params (LookSpeed :type Float%20%28single-precision%29))
  (Variables|Default|SetLookSpeed LookSpeed))

(fn SetMoveSpeed
  (params (MoveSpeed :type Float%20%28single-precision%29))
  (Variables|Default|SetMoveSpeed MoveSpeed))