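; BP_InventorySystem is an Actor Blueprint that holds a size-limited inventory of items.
; AddToInventory appends an item and increments a manual size counter only while it is below MaxInventorySize.
; CheckIfContains linearly searches the Inventory array for a match.
; UseItem only removes the item and decrements the counter without checking it was present, and the event graph is empty.
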(event EventBeginPlay)

(event EventTick
  (params (DeltaSeconds :type Float%20%28single-precision%29)))

(fn ConstructionScript)

(fn AddtoInventory
  (params (NewItem :type String))
  (if (> (Variables|Default|GetMaxInventorySize) (Variables|Default|GetInventorySize))
    (Utilities|Array|Add (Variables|Default|GetInventory) NewItem)
    (Math|Integer|IncrementInt (Variables|Default|GetInventorySize))))

(fn CheckifContains
  (params (Item :type String))
  (for _array_element (Variables|Default|GetInventory)
    (if (Utilities|Enum|Equal(Enum) _array_element Item)
      (return true)))
  (return false))

(fn UseItem
  (params (Item :type String))
  (Utilities|Array|RemoveItem (Variables|Default|GetInventory) Item)
  (Variables|Default|SetInventorySize (- (Variables|Default|GetInventorySize) 1)))